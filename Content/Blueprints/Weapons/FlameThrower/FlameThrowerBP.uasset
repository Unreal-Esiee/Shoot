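; FlameThrowerBP is a flamethrower weapon Blueprint that spawns flame projectiles when fired.
; Its Fire event takes the firing character and spawns a FlameThrowerProjectile at the Sphere component's position plus GunOffset rotated by the first-person camera.
; The projectile faces along the camera's rotation and always spawns regardless of collision.
; Each shot plays the FlameShot sound at the weapon's location.
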(event EventFire
  (params (Character :type First%20Person%20Character%20Object%20Reference))
  (bind _firstpersoncamera (Variables|/Game/Blueprints/FirstPerson/Blueprints/FirstPersonCharacter.FirstPersonCharacter_C|GetFirstPersonCamera Character))
  (bind _returnvalue (Transformation|GetWorldRotation _firstpersoncamera))
  (Game|SpawnActorfromClass "/Game/Blueprints/Weapons/FlameThrower/FlameThrowerProjectile.FlameThrowerProjectile_C" (Math|Transform|MakeTransform (+ (Transformation|GetWorldLocation (Variables|Default|GetSphere)) (Math|Vector|RotateVector (Variables|Default|GetGunOffset) _returnvalue)) _returnvalue) "AlwaysSpawn" 0 0) ; Spawn projectile
  (Audio|PlaySoundatLocation "/Game/Blueprints/Weapons/FlameThrower/flameShot.flameShot" (Transformation|GetActorLocation) "0, 0, 0" 1.0 1.0 0.0 0 0 0) ; Play firing sound
)

(fn ConstructionScript)
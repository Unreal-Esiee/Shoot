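; NPC AI controller that steers its pawn toward the first IA_Target_BP actor found in the level.
; On BeginPlay it sets up the NPC_BB blackboard, seeds MoveLocation and runs the NPC_BT behavior tree.
; Every Tick it searches for the target again and rewrites MoveLocation with a random reachable point around it.
; A TODO flags this per-frame detection method for replacement.
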(event EventBeginPlay
  (bind _blackboardcomponent (Class|AIController|UseBlackboard "/Game/Blueprints/NPC/NPC_BB.NPC_BB"))
  (Variables|Default|SetCurrentBlackBoard _blackboardcomponent)
  (bind _outactors (Actor|GetAllActorsOfClass "/Game/Blueprints/NPC/IA_Target_BP.IA_Target_BP_C"))
  (AI|Components|Blackboard|SetValueasVector (Variables|Default|GetCurrentBlackBoard) (Utilities|Name|MakeLiteralName "MoveLocation") (.RandomLocation (AI|Navigation|GetRandomReachablePointinRadius (Transformation|GetActorLocation (Utilities|Array|Get(acopy) _outactors)) 0.0 0 0)))
  (AI|RunBehaviorTree "/Game/Blueprints/NPC/NPC_BT.NPC_BT"))

(event EventTick
  (params (DeltaSeconds :type Float%20%28single-precision%29))
  ;[1 1 1] TODO : Changer la méthode de détection
  (bind _outactors (Actor|GetAllActorsOfClass "/Game/Blueprints/NPC/IA_Target_BP.IA_Target_BP_C"))
  (AI|Components|Blackboard|SetValueasVector (Variables|Default|GetCurrentBlackBoard) (Utilities|Name|MakeLiteralName "MoveLocation") (.RandomLocation (AI|Navigation|GetRandomReachablePointinRadius (Transformation|GetActorLocation (Utilities|Array|Get(acopy) _outactors)) 0.0 0 0))))

(fn ConstructionScript)
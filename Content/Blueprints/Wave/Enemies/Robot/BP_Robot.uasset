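; BP_Robot is a wave enemy that damages the player on attack-zone overlap, then dies.
; It registers with FirstPersonGameMode's alive count on spawn and decrements it on death, triggering a remaining-enemy check.
; Health changes update a hidden widget, briefly shown after non-lethal hits.
; Lethal damage awards the player money and, after calling Die, has a small chance to spawn a random pickup.
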(event OnComponentBeginOverlap(AttackZone)
  (params (OverlappedComponent :type Primitive%20Component%20Object%20Reference) (OtherActor :type Actor%20Object%20Reference) (OtherComp :type Primitive%20Component%20Object%20Reference) (OtherBodyIndex :type Integer) (bFromSweep :type Boolean) (SweepResult :type Hit%20Result%20Structure%20%28by%20ref%29))
  (bind _asfirst_person_character (Utilities|Casting|CastToFirstPersonCharacter OtherActor))
  (Default|LoseLife _asfirst_person_character (Variables|Default|GetDamage))
  (CallFunction|Die))

(event Custom|Drop%20Loot
  (Game|SpawnActorfromClass (.OutItem (Utilities|Array|Random (Variables|Default|GetPossiblesPickups))) (Transformation|GetActorTransform) "Undefined" 0 0))

(event Custom|Die
  (bind _asfirst_person_game_mode (Utilities|Casting|CastToFirstPersonGameMode (Game|GetGameMode)))
  (Math|Integer|DecrementInt (Variables|/Game/Blueprints/FirstPerson/Blueprints/FirstPersonGameMode.FirstPersonGameMode_C|GetEnemyAlive _asfirst_person_game_mode)
    (:%20%20
      (Default|CheckEnemyLeft _asfirst_person_game_mode)
      (Actor|DestroyActor))))

(event EventGainLife
  (params (Gain :type Float%20%28single-precision%29))
  (bind _output_get (Variables|Default|SetHealth (+ (Variables|Default|GetHealth) Gain)))
  (Variables|/Game/Blueprints/Wave/NPC_Healt_Widget.NPC_Healt_Widget_C|SetHealthWidget (Variables|Default|GetHealthWidgetREF) _output_get))

(event EventLoseLife
  (params (Damage :type Float%20%28single-precision%29))
  (bind _output_get (Variables|Default|SetHealth (- (Variables|Default|GetHealth) Damage)))
  (if (<= _output_get 0.0)
    (Class|MoneyInterface|EarnMoney(Message) (Game|GetPlayerCharacter 0) 10)
    (CallFunction|Die)
    (if (>= (Math|Random|RandomFloat) 0.9)
      (CallFunction|DropLoot))
    (else
      (Utilities|FlowControl|Sequence
        (:then_0
          (Variables|/Game/Blueprints/Wave/NPC_Healt_Widget.NPC_Healt_Widget_C|SetHealthWidget (Variables|Default|GetHealthWidgetREF) (stale EventGainLife _output_get)))
        (:then_1
          (Widget|SetVisibility (Variables|Default|GetHealthWidgetREF) "Visible")
          (Utilities|FlowControl|Delay 2.0)
          (Widget|SetVisibility (Variables|Default|GetHealthWidgetREF) "Hidden"))))))

(event EventBeginPlay
  (Utilities|FlowControl|Sequence
    (:then_0
      (bind _asfirst_person_game_mode (Utilities|Casting|CastToFirstPersonGameMode (Game|GetGameMode)))
      (Math|Integer|IncrementInt (Variables|/Game/Blueprints/FirstPerson/Blueprints/FirstPersonGameMode.FirstPersonGameMode_C|GetEnemyAlive _asfirst_person_game_mode)))
    (:then_1
      (bind _asnpc_healt_widget (Utilities|Casting|CastToNPC_Healt_Widget (UserInterface|GetUserWidgetObject (Variables|Default|GetHealthWidget))))
      (bind _output_get (Variables|Default|SetHealthWidgetREF _asnpc_healt_widget))
      (bind _output_get_2 (Variables|/Game/Blueprints/Wave/NPC_Healt_Widget.NPC_Healt_Widget_C|SetInitialWidget _output_get (Variables|Default|GetHealth)))
      (Variables|/Game/Blueprints/Wave/NPC_Healt_Widget.NPC_Healt_Widget_C|SetHealthWidget _output_get _output_get_2)
      (Widget|SetVisibility _output_get "Hidden"))))

(fn ConstructionScript)
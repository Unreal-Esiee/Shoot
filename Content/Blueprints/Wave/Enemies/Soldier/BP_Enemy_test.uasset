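; Test soldier enemy for the wave system that damages the player when they overlap its AttackZone, then dies in the same hit.
; BeginPlay registers it in FirstPersonGameMode's alive count and sets up a hidden health widget.
; Health changes update the widget, which shows for two seconds after non-lethal damage.
; Both death paths decrement the count, trigger the game mode's remaining-enemy check, destroy the actor and spawn a health-mesh pickup.
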(event OnComponentBeginOverlap(AttackZone)
  (params (OverlappedComponent :type Primitive%20Component%20Object%20Reference) (OtherActor :type Actor%20Object%20Reference) (OtherComp :type Primitive%20Component%20Object%20Reference) (OtherBodyIndex :type Integer) (bFromSweep :type Boolean) (SweepResult :type Hit%20Result%20Structure%20%28by%20ref%29))
  (bind _asfirst_person_character (Utilities|Casting|CastToFirstPersonCharacter OtherActor))
  (Default|LoseLife _asfirst_person_character (Variables|Default|GetDamage))
  (bind _asfirst_person_game_mode (Utilities|Casting|CastToFirstPersonGameMode (Game|GetGameMode)))
  (Math|Integer|DecrementInt (Variables|/Game/Blueprints/FirstPerson/Blueprints/FirstPersonGameMode.FirstPersonGameMode_C|GetEnemyAlive _asfirst_person_game_mode)
    (:%20%20
      (Default|CheckEnemyLeft _asfirst_person_game_mode)
      (Actor|DestroyActor)
      (bind _returnvalue (Game|SpawnActorfromClass "/Game/Blueprints/Pickups/PickUp_BP.PickUp_BP_C" (Transformation|GetActorTransform) "Undefined" 0 0))
      (Variables|/Game/Blueprints/Pickups/PickUp_BP.PickUp_BP_C|SetItem_Type _returnvalue "NewEnumerator0")
      (Variables|/Game/Blueprints/Pickups/PickUp_BP.PickUp_BP_C|SetItem_Mesh _returnvalue "/Game/Blueprints/Pickups/HealthMesh.HealthMesh"))))

(event EventGainLife
  (params (Gain :type Float%20%28single-precision%29))
  (Variables|Default|SetHealth (+ (Variables|Default|GetHealth) Gain))
  (Variables|/Game/Blueprints/Wave/NPC_Healt_Widget.NPC_Healt_Widget_C|SetHealthWidget (Variables|Default|GetHealthWidgetREF) (stale EventLoseLife _output_get)))

(event EventLoseLife
  (params (Damage :type Float%20%28single-precision%29))
  (bind _output_get (Variables|Default|SetHealth (- (Variables|Default|GetHealth) Damage)))
  (Utilities|FlowControl|Sequence
    (:then_0
      (Variables|/Game/Blueprints/Wave/NPC_Healt_Widget.NPC_Healt_Widget_C|SetHealthWidget (Variables|Default|GetHealthWidgetREF) _output_get))
    (:then_1
      (if (<= _output_get 0.0)
        (bind _asfirst_person_game_mode (Utilities|Casting|CastToFirstPersonGameMode (Game|GetGameMode)))
        (Math|Integer|DecrementInt (Variables|/Game/Blueprints/FirstPerson/Blueprints/FirstPersonGameMode.FirstPersonGameMode_C|GetEnemyAlive _asfirst_person_game_mode)
          (:%20%20
            (Default|CheckEnemyLeft _asfirst_person_game_mode)
            (Actor|DestroyActor)
            (bind _returnvalue (Game|SpawnActorfromClass "/Game/Blueprints/Pickups/PickUp_BP.PickUp_BP_C" (Transformation|GetActorTransform) "Undefined" 0 0))
            (Variables|/Game/Blueprints/Pickups/PickUp_BP.PickUp_BP_C|SetItem_Type _returnvalue "NewEnumerator0")
            (Variables|/Game/Blueprints/Pickups/PickUp_BP.PickUp_BP_C|SetItem_Mesh _returnvalue "/Game/Blueprints/Pickups/HealthMesh.HealthMesh")))
        (else
          (Widget|SetVisibility (Variables|Default|GetHealthWidgetREF) "Visible")
          (Utilities|FlowControl|Delay 2.0)
          (Widget|SetVisibility (Variables|Default|GetHealthWidgetREF) "Hidden"))))))

(event EventBeginPlay
  (Utilities|FlowControl|Sequence
    (:then_0
      (bind _asfirst_person_game_mode (Utilities|Casting|CastToFirstPersonGameMode (Game|GetGameMode)))
      (Math|Integer|IncrementInt (Variables|/Game/Blueprints/FirstPerson/Blueprints/FirstPersonGameMode.FirstPersonGameMode_C|GetEnemyAlive _asfirst_person_game_mode)))
    (:then_1
      (bind _asnpc_healt_widget (Utilities|Casting|CastToNPC_Healt_Widget (UserInterface|GetUserWidgetObject (Variables|Default|GetHealthWidget))))
      (bind _output_get (Variables|Default|SetHealthWidgetREF _asnpc_healt_widget))
      (Variables|/Game/Blueprints/Wave/NPC_Healt_Widget.NPC_Healt_Widget_C|SetInitialWidget _output_get (Variables|Default|GetHealth))
      (Variables|/Game/Blueprints/Wave/NPC_Healt_Widget.NPC_Healt_Widget_C|SetHealthWidget _output_get 0.0)
      (Widget|SetVisibility _output_get "Hidden"))))

(fn ConstructionScript)
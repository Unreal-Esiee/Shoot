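; Enemy spawner actor that spawns escalating waves of AI at its location when the FirstPersonGameMode's respawn-enemy event fires.
; A delayed loop spawns batches of eight pawns, drawing pawn class and behavior tree at random from the Enemies array and ignoring collision.
; After each wave it raises the increment and adds it to the enemy count, so waves grow at an accelerating rate.
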(event Custom|SpawnEnemy
  (bind _enemyspawnincrement (Variables|Default|GetEnemySpawnIncrement))
  (bind _enemies (Variables|Default|GetEnemies))
  (bind _outitem (Utilities|Array|Random _enemies))
  (Utilities|ForLoopwithDelay 0 (/ (Variables|Default|GetEnemySpawned) 8) 0.8
    (:Loop%20Body
      (for _index (range 0 7)
        (AI|SpawnAIFromClass (.pawnclass _outitem) (.behavoirtree _outitem) (Transformation|GetActorLocation) "0, 0, 0" true 0)))
    (:Completed
      (Math|Integer|IncrementInt _enemyspawnincrement
        (:%20%20
          (Variables|Default|SetEnemySpawned (+ _enemyspawnincrement (Variables|Default|GetEnemySpawned))))))))

(event EventBeginPlay
  (bind _asfirst_person_game_mode (Utilities|Casting|CastToFirstPersonGameMode (Game|GetGameMode)))
  (EventDispatchers|BindEventtoRespawnEnemy _asfirst_person_game_mode (delegate Custom|SpawnEnemy)))

(fn ConstructionScript)